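; TestWRBP is a test actor for writing and reading text files as string arrays.
; BeginPlay enables input from the first player controller so two debug keys work.
; Key 1 saves a hardcoded sample array with overwrite and prints the result; key 2 reads another file and prints each line prefixed by its index.
; Both file locations are hardcoded absolute paths on a local drive.
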(event `self.ReceiveBeginPlay`
  (`self.EnableInput` (`GameplayStatics.GetPlayerController` 0)))

(event `Key|One`
  (params (Key :type "Key Structure"))
  (:`Pressed`
    (bind _returnvalue (`MyNewBFL.SaveTextArray` "D:\\code\\codes\\ueProject\\MyProject\\ACProject" "test.txt" (`|MakeArray` "rowenci" "hello" "world!") true))
    (`KismetSystemLibrary.PrintString` (`KismetStringLibrary.Conv_BoolToString` _returnvalue))))

(event `Key|Two`
  (params (Key :type "Key Structure"))
  (:`Pressed`
    (bind _returnvalue (`MyNewBFL.ReadTextArray` "D:\\code\\codes\\Data\\print" "0.txt"))
    (for (_array_element _array_index) _returnvalue
      (`KismetSystemLibrary.PrintString` (`KismetStringLibrary.Concat_StrStr` (`KismetStringLibrary.Concat_StrStr` (`KismetStringLibrary.BuildString_Int` "" "" _array_index) " ") _array_element)))))

(fn `UserConstructionScript`)